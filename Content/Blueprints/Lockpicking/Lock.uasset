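; Lockpicking minigame on a 3x3 grid: find and unlock every breaking point before wall hits wear out the pick.
; SetField builds the puzzle from a random wall preset, shuffled points scaled by Difficulty and Hacking skill, and random 90-degree rotations.
; Axis input accumulates until it crosses CellSize, then steps the pick through wall checks; left-click unlocks the current point.
; Feedback is only sounds and debug prints.
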(event `self.ReceiveBeginPlay`
  ;[1 1 1] Setup field
  (`self.SetField` (`self.Difficulty`) (`self.Hacking`))
  (`KismetSystemLibrary.PrintString` (`KismetStringLibrary.Concat_StrStr` "Breaking points left: " (`KismetStringLibrary.Conv_IntToString` (`KismetArrayLibrary.Array_Length` (`self.BreakingPoints`)))) true true (struct :`G` 0.66 :`B` 1.0 :`A` 1.0) 2000.0))

(event `InputAxis|Forward`
  (params (AxisValue :type "Float (single-precision)"))
  ;[1 1 1] Receive input and check for lockpick move
  (set `self.CellOffset` (+ (`KismetMathLibrary.MakeVector2D` 0.0 AxisValue) (`self.CellOffset`)))
  (`self.CheckMove` :!label _label))

(event `InputAxis|Right`
  (params (AxisValue :type "Float (single-precision)"))
  ;[1 1 1] Receive input and check for lockpick move
  (set `self.CellOffset` (+ (`KismetMathLibrary.MakeVector2D` AxisValue) (`self.CellOffset`)))
  (goto _label))

(event `Key|LeftMouseButton`
  (params (Key :type "Key Structure"))
  ;[1 1 1] Unlocking breaking points
  (:`Pressed`
    (bind _isbreakingpoint (`self.CheckForBreakingPoint`))
    (if _isbreakingpoint
      (`self.UnlockBreakingPoint` (`self.LockpickPosition`))
      (`KismetSystemLibrary.PrintString` "Unlocked!" true true (struct :`R` 1.0 :`B` 0.802035 :`A` 1.0) 10000.0)
      (`KismetSystemLibrary.PrintString` (`KismetStringLibrary.Concat_StrStr` "Breaking points left: " (`KismetStringLibrary.Conv_IntToString` (`KismetArrayLibrary.Array_Length` (`self.BreakingPoints`)))) true true (struct :`G` 0.66 :`B` 1.0 :`A` 1.0) 2000.0)
      (`GameplayStatics.PlaySound2D` "/Game/Sounds/sfx_sounds_interaction12.sfx_sounds_interaction12")
      (if (== (`KismetArrayLibrary.Array_Length` (`self.BreakingPoints`)) 0)
        (`self.Unlocked`))
      (else
        (`KismetSystemLibrary.PrintString` "Bad attempt" true true (struct :`R` 1.0 :`G` 0.453206 :`A` 1.0) 2000.0)))))

(fn `AddIntPoints`
  (params (Point1 :type "IntPoint Structure") (Point2 :type "IntPoint Structure"))
  (returns (PointsSum :type "IntPoint Structure"))
  (locals (X :type Integer) (Y :type Integer))
  (bind (_x _y) (break `IntPoint` Point1))
  (bind (_x_2 _y_2) (break `IntPoint` Point2))
  (return (make `IntPoint` (+ _x _x_2) (+ _y _y_2))))

(fn `CheckForBreakingPoint`
  (returns (IsBreakingPoint :type Boolean))
  (for _array_element (`self.BreakingPoints`)
    (bind _equals (`self.CompareIntPoints` _array_element (`self.LockpickPosition`)))
    (if _equals
      (return true)))
  (return false))

(fn `CheckMove`
  (bind _cellsize (`self.CellSize`))
  (bind (_x _y) (`KismetMathLibrary.BreakVector2D` (`self.CellOffset`)))
  (bind _returnvalue (* -1 _cellsize))
  (if (< _x _returnvalue)
    (`self.MoveLockpick` (make `IntPoint` -1))
    ;[1 1 1] Debug
    (`KismetSystemLibrary.PrintString` "Moving left..." true true (struct :`R` 0.911063 :`G` 1.0 :`A` 1.0) 1000.0)
    (elif (> _x _cellsize)
      (`self.MoveLockpick` (make `IntPoint` 1))
      (`KismetSystemLibrary.PrintString` "Moving right..." true true (struct :`R` 0.911063 :`G` 1.0 :`A` 1.0) 1000.0)
      (elif (< _y _returnvalue)
        (`self.MoveLockpick` (make `IntPoint` 0 1))
        (`KismetSystemLibrary.PrintString` "Moving down..." true true (struct :`R` 0.911063 :`G` 1.0 :`A` 1.0) 1000.0)
        (elif (> _y _cellsize)
          (`self.MoveLockpick` (make `IntPoint` 0 -1))
          (`KismetSystemLibrary.PrintString` "Moving up..." true true (struct :`R` 0.911063 :`G` 1.0 :`A` 1.0) 1000.0))))))

(fn `CheckWalls`
  (params (CurrentPosition :type "IntPoint Structure") (NewPosition :type "IntPoint Structure"))
  (returns (WallHit :type Boolean))
  (locals (CurrentPos :type "IntPoint Structure") (NewPos :type "IntPoint Structure"))
  (bind (_x _y) (break `IntPoint` NewPosition))
  ;[1 1 1] Check for outer walls hit
  (set `local.CurrentPos` CurrentPosition)
  (set `local.NewPos` NewPosition)
  (if (or (> _x 2) (< _x 0) (> _y 2) (< _y 0))
    (return true)
    (else
      ;[1 1 1] Check for inner walls hit
      (for _array_element (`self.Walls`)
        (bind (_fromside _toside) (break `/Game/Blueprints/Lockpicking/Wall` _array_element))
        (bind _equals (`self.CompareIntPoints` _fromside (`local.CurrentPos`)))
        (bind _equals_2 (`self.CompareIntPoints` _toside (`local.NewPos`)))
        (bind _equals_3 (`self.CompareIntPoints` _fromside (`local.NewPos`)))
        (bind _equals_4 (`self.CompareIntPoints` _toside (`local.CurrentPos`)))
        (if (or (and _equals_2 _equals) (and _equals_3 _equals_4))
          (return true)))
      (return false))))

(fn `CompareIntPoints`
  (params (Point1 :type "IntPoint Structure") (Point2 :type "IntPoint Structure"))
  (returns (Equals :type Boolean))
  (bind (_x _y) (break `IntPoint` Point1))
  (bind (_x_2 _y_2) (break `IntPoint` Point2))
  (return (and (== _x _x_2) (== _y _y_2))))

(fn `MoveLockpick`
  (params (Direction :type "IntPoint Structure"))
  (locals (NewPosition :type "IntPoint Structure"))
  (bind _wearscale (`self.WearScale`))
  ;[1 1 1] Move lockpick
  (bind _pointssum (`self.AddIntPoints` Direction (`self.LockpickPosition`)))
  (set `local.NewPosition` _pointssum)
  (set `self.CellOffset` (0.0 0.0))
  (bind _wallhit (`self.CheckWalls` (`self.LockpickPosition`) (`local.NewPosition`)))
  (if _wallhit
    ;[1 1 1] If lockpick hit the wall
    (`KismetSystemLibrary.PrintString` "Wall hit!" true true (struct :`R` 1.0 :`B` 0.029149 :`A` 1.0) 10000.0)
    (`GameplayStatics.PlaySound2D` "/Game/Sounds/sfx_sounds_button8.sfx_sounds_button8")
    (`/Engine/EditorBlueprintResources/StandardMacros.DecrementInt` _wearscale
      (:`  `
        (if (<= _wearscale 0)
          (`KismetSystemLibrary.PrintString` "YOU LOST!" true true (struct :`R` 1.0 :`B` 0.113724 :`A` 1.0) 1000.0)
          (`self.DisableInput` (`GameplayStatics.GetPlayerController` 0))
          (else
            (`KismetSystemLibrary.PrintString` (`KismetStringLibrary.Concat_StrStr` "Wear scale left: " (`KismetStringLibrary.Conv_IntToString` (`self.WearScale`))) true true (struct :`G` 0.66 :`B` 1.0 :`A` 1.0) 2000.0)))))
    (else
      (bind _output_get (set `self.LockpickPosition` (`local.NewPosition`)))
      (bind _isbreakingpoint (`self.CheckForBreakingPoint`))
      (if _isbreakingpoint
        ;[1 1 1] If lockpick hit breaking point
        (`GameplayStatics.PlaySound2D` "/Game/Sounds/sfx_coin_double7.sfx_coin_double7")
        (`KismetSystemLibrary.PrintString` "Breaking point!" true true (struct :`R` 0.004252 :`G` 1.0 :`A` 1.0) 1000.0))
      (bind (_x _y) (break `IntPoint` _output_get))
      (`KismetSystemLibrary.PrintString` (`KismetStringLibrary.Concat_StrStr` (`KismetStringLibrary.Conv_IntToString` _x) " : " (`KismetStringLibrary.Conv_IntToString` _y)) true true (struct :`G` 0.66 :`B` 1.0 :`A` 1.0) 1000.0))))

(fn `RotateField90`
  ;[1 1 1] Rotate walls
  (for _index (range (+ (`KismetArrayLibrary.Array_Length` (`self.Walls`)) 1))
    (bind (_fromside _toside) (break `/Game/Blueprints/Lockpicking/Wall` (`|GetArrayItem` (`self.Walls`) _index)))
    (`KismetArrayLibrary.Array_Set` (`self.Walls`) _index (make `/Game/Blueprints/Lockpicking/Wall` (`self.RotatePoint90` _fromside) (`self.RotatePoint90` _toside))))
  ;[1 1 1] Rotate breaking points
  (for _index_2 (range (+ (`KismetArrayLibrary.Array_Length` (`self.BreakingPoints`)) 1))
    (`KismetArrayLibrary.Array_Set` (`self.BreakingPoints`) _index_2 (`self.RotatePoint90` (`|GetArrayItem` (`self.BreakingPoints`) _index_2)))))

(fn `RotatePoint90`
  (params (Point :type "IntPoint Structure"))
  (returns (RotatedPoint :type "IntPoint Structure"))
  (bind (_x _y) (break `IntPoint` Point))
  (return (make `IntPoint` (- 2 _y) _x)))

(fn `SetField`
  (params (BreakingPointsNumber :type Integer :default 1) (Hacking :type Integer))
  (locals (TempRow :type "Array of Boolean") (BasicFields :type "Array of /Game/Blueprints/Lockpicking/WallsArray Structure") (BreakingPoints_ :type "Array of IntPoint Structure") (BP_Number :type Integer :default 1) (AdditionalBreakingPoints :type "Array of IntPoint Structure"))
  (bind _additionalbreakingpoints (`local.AdditionalBreakingPoints`))
  ;[1 1 1] Setup walls and break points number
  (set `local.BP_Number` BreakingPointsNumber)
  (if (>= Hacking 3)
    (bind _result (`/Engine/EditorBlueprintResources/StandardMacros.DecrementInt` (`local.BP_Number`))
      (:`  `
        (if (== _result 0)
          (`self.Unlocked`)
          (return)
          (else
            _)))))
  (set `self.Walls` (`.Walls_3_67EE097E4BB94377D24693A157E9211C` (break `/Game/Blueprints/Lockpicking/WallsArray` (`|GetArrayItem` (`local.BasicFields`) (`KismetMathLibrary.RandomInteger` 3)))))
  ;[1 1 1] Shuffle breaking points and add additional one if (Difficulty == 4)
  (`KismetArrayLibrary.Array_Shuffle` (`local.BreakingPoints_`))
  (if (== (`local.BP_Number`) 4)
    (`KismetArrayLibrary.Array_Add` (`local.BreakingPoints_`) (`|GetArrayItem` _additionalbreakingpoints (`KismetMathLibrary.RandomInteger` (`KismetArrayLibrary.Array_Length` _additionalbreakingpoints)))))
  ;[1 1 1] Setup breaking points
  (for _index (range (`local.BP_Number`))
    (`KismetArrayLibrary.Array_Add` (`self.BreakingPoints`) (`|GetArrayItem` (`local.BreakingPoints_`) _index)))
  ;[1 1 1] Rotate field
  (for _ (range (+ (`KismetMathLibrary.RandomInteger` 4) 1))
    (`self.RotateField90`)))

(fn `UnlockBreakingPoint`
  (params (Position :type "IntPoint Structure"))
  (`KismetArrayLibrary.Array_RemoveItem` (`self.BreakingPoints`) Position))

(fn `Unlocked`
  (`KismetSystemLibrary.PrintString` "YOU WIN!" true true (struct :`R` 1.0 :`B` 0.624415 :`A` 1.0) 1000.0)
  (`self.DisableInput` (`GameplayStatics.GetPlayerController` 0)))

(fn `UserConstructionScript`)