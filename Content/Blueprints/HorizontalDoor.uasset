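; Horizontal sliding double door Blueprint with OpenDoor and CloseDoor events.
; OpenDoor plays the DoorOpening timeline, whose DoorOffset track moves LeftDoor and RightDoor in opposite directions, and CloseDoor reverses that timeline.
; Each update applies the offset to the doors' current relative locations rather than cached start positions, so movement accumulates frame by frame.
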(event `self.OpenDoor`
  (bind _leftdoor (`self.LeftDoor`))
  (bind _rightdoor (`self.RightDoor`))
  (bind (_direction _dooroffset) (`Timeline|DoorOpening` :!label _label)
    (:`Update`
      (`SceneComponent.K2_SetRelativeLocation` _leftdoor (+ _dooroffset (`SceneComponent.RelativeLocation` _leftdoor)) false false)
      (`SceneComponent.K2_SetRelativeLocation` _rightdoor (- (`SceneComponent.RelativeLocation` _rightdoor) _dooroffset) false false))))

(event `self.CloseDoor`
  (goto _label :!via `Reverse`))

(fn `UserConstructionScript`
  (`parent.UserConstructionScript`))